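; BP_door is an interactive door that the player opens and closes with the Interact input while near it.
; Overlapping the Trigger component enables input for player 0 and shows a prompt widget once, while leaving disables input, removes the widget and resets the gate.
; A FlipFlop alternately plays and reverses the Rotation timeline, which adds yaw to the rotation captured at BeginPlay to swing the whole actor.
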(event `self.Trigger.OnComponentBeginOverlap`
  (params (OverlappedComponent :type "PrimitiveComponent Object Reference") (OtherActor :type "Actor Object Reference") (OtherComp :type "PrimitiveComponent Object Reference") (OtherBodyIndex :type Integer) (bFromSweep :type Boolean) (SweepResult :type "HitResult Structure (by ref)"))
  ;[1 1 1] Triggerbox
  (`self.EnableInput` (`GameplayStatics.GetPlayerController` 0))
  (`/Engine/EditorBlueprintResources/StandardMacros.DoOnce` false :!label _label
    (:`Completed`
      (bind _returnvalue (`|CreateWidget` "/Game/Blueprints/Doors/MessageNearTheDoor.MessageNearTheDoor_C" (`GameplayStatics.GetPlayerController` 0)))
      (`UserWidget.AddToViewport` _returnvalue 0))))

(event `self.Trigger.OnComponentEndOverlap`
  (params (OverlappedComponent :type "PrimitiveComponent Object Reference") (OtherActor :type "Actor Object Reference") (OtherComp :type "PrimitiveComponent Object Reference") (OtherBodyIndex :type Integer))
  ;[1 1 1] Triggerbox
  (`self.DisableInput` (`GameplayStatics.GetPlayerController` 0))
  (`Widget.RemoveFromParent` (stale `self.Trigger.OnComponentBeginOverlap` _returnvalue))
  (goto _label :!via `Reset`))

(event `InputAction|Interact`
  (params (Key :type "Key Structure"))
  ;[1 1 1] Configure rotator
  (:`Pressed`
    (`/Engine/EditorBlueprintResources/StandardMacros.FlipFlop`
      (:`A`
        (bind (_direction _door_rotation) (`Timeline|Rotation` :!label _label_2)
          (:`Update`
            (`self.K2_SetActorRelativeRotation` (`KismetMathLibrary.ComposeRotators` (`KismetMathLibrary.MakeRotator` 0.0 0.0 _door_rotation) (`self.Porte_ini`))))))
      (:`B`
        (goto _label_2 :!via `Reverse`)))))

(event `self.ReceiveBeginPlay`
  ;[1 1 1] Init
  (set `self.Porte_ini` (`self.K2_GetActorRotation`)))

(fn `UserConstructionScript`)
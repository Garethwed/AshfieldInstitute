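; Interactable drawer Blueprint that shows a prompt when approached and opens on the Interact input.
; Box overlap enables input and creates the MessageNearDrawer widget once; leaving removes it and resets the gate.
; Interact disables input, removes the prompt and plays the Open timeline, which sets the drawer's relative location through a zero-alpha lerp.
; The timeline update also flags the drawer open and spawns an inspectable object once at hardcoded coordinates.
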(event `self.Box.OnComponentBeginOverlap`
  (params (OverlappedComponent :type "PrimitiveComponent Object Reference") (OtherActor :type "Actor Object Reference") (OtherComp :type "PrimitiveComponent Object Reference") (OtherBodyIndex :type Integer) (bFromSweep :type Boolean) (SweepResult :type "HitResult Structure (by ref)"))
  ;[1 1 1] Triggerbox to spawn Open menu
  (`self.EnableInput` (`GameplayStatics.GetPlayerController` 0))
  (`/Engine/EditorBlueprintResources/StandardMacros.DoOnce` false :!label _label
    (:`Completed`
      (if (`self.IsDrawerOpen`)
        (`Widget.RemoveFromParent` (stale `self.Box.OnComponentBeginOverlap` _returnvalue) :!label _label_2)
        (goto _label :!via `Reset`)
        (else
          (bind _returnvalue (`|CreateWidget` "/Game/Blueprints/Doors/MessageNearDrawer.MessageNearDrawer_C" (`GameplayStatics.GetPlayerController` 0)))
          (`UserWidget.AddToViewport` _returnvalue 0))))))

(event `self.Box.OnComponentEndOverlap`
  (params (OverlappedComponent :type "PrimitiveComponent Object Reference") (OtherActor :type "Actor Object Reference") (OtherComp :type "PrimitiveComponent Object Reference") (OtherBodyIndex :type Integer))
  ;[1 1 1] Triggerbox to spawn Open menu
  (goto _label_2))

(event `InputAction|Interact`
  (params (Key :type "Key Structure"))
  ;[1 1 1] open drawer, disable open menu widget and spawn interactable object
  (:`Pressed`
    (`self.DisableInput` (`GameplayStatics.GetPlayerController` 0))
    (`Widget.RemoveFromParent` (stale `self.Box.OnComponentBeginOverlap` _returnvalue))
    (bind (_direction _newtrack_0) (`Timeline|Open`)
      (:`Update`
        (`SceneComponent.K2_SetRelativeLocation` (`self.Drawer`) (`KismetMathLibrary.VLerp` (0.0 50.0 0.0) (`KismetMathLibrary.Conv_DoubleToVector` _newtrack_0)) false false)
        (set `self.IsDrawerOpen` true)
        (`/Engine/EditorBlueprintResources/StandardMacros.DoOnce` false
          (:`Completed`
            (`|SpawnActorFromClass` "/Game/Blueprints/ItemInteractionV2/InspectableObj_Child1.InspectableObj_Child1_C" (`KismetMathLibrary.MakeTransform` (-1171.0 697.0 185.0) (struct) (0.7 0.7 0.4)) "Undefined" "OverrideRootScale" null null)))))))

(fn `UserConstructionScript`)